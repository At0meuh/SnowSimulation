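; BP_Capture is a snow system actor that keeps an orthographic scene capture following the player character in XY.
; Each tick, MoveCapture moves it to the player position snapped to render-target pixel size, a technique that avoids sub-pixel shifts.
; It publishes capture size at BeginPlay and location each tick to MPC_Capture for materials.
; DrawToPersistant, meant to draw the movement offset into RT_Persistant, and its dynamic material setup never run.
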(event `self.ReceiveBeginPlay`
  (`KismetMaterialLibrary.SetScalarParameterValue` "/Game/SnowSystem/Material/MPC_Capture.MPC_Capture" "CaptureSize" (`SceneCaptureComponent2D.OrthoWidth` (`self.SceneCaptureComponent2D`))))

(event `self.ReceiveTick`
  (params (DeltaSeconds :type "Float (single-precision)"))
  (`self.MoveCapture`))

(fn `DrawToPersistant`
  (bind _orthowidth (`SceneCaptureComponent2D.OrthoWidth` (`self.SceneCaptureComponent2D`)))
  (bind (_returnvalue_x _returnvalue_y) (`KismetMathLibrary.BreakVector2D` (/ (`self.MoveOffset`) (`KismetMathLibrary.MakeVector2D` _orthowidth _orthowidth))))
  (`MaterialInstanceDynamic.SetVectorParameterValue` (`self.DrawMaterial`) "None" (make `LinearColor` _returnvalue_x _returnvalue_y 0.0 1.0))
  (`KismetRenderingLibrary.DrawMaterialToRenderTarget` "/Game/SnowSystem/RenderTarget/RT_Persistant.RT_Persistant" (`self.DrawMaterial`)))

(fn `MoveCapture`
  (bind (_returnvalue_x _returnvalue_y) (`KismetMathLibrary.BreakVector` (`self.K2_GetActorLocation` (`GameplayStatics.GetPlayerCharacter` 0))))
  (bind _output_get (set `self.MoveOffset` (`KismetMathLibrary.MakeVector2D` (.x (- (`self.SnapToPixelWorldSize` _returnvalue_x _returnvalue_y (* (`SceneCaptureComponent2D.OrthoWidth` (`self.SceneCaptureComponent2D`)) (/ 1.0 (`self.RenderTargetResolution`)))) (`self.K2_GetActorLocation`))) (.y (- (`self.SnapToPixelWorldSize` _returnvalue_x _returnvalue_y (* (`SceneCaptureComponent2D.OrthoWidth` (`self.SceneCaptureComponent2D`)) (/ 1.0 (`self.RenderTargetResolution`)))) (`self.K2_GetActorLocation`))))))
  (bind (_x _y) (`KismetMathLibrary.BreakVector2D` _output_get))
  (`self.K2_AddActorWorldOffset` (`KismetMathLibrary.MakeVector` _x _y))
  (`KismetMaterialLibrary.SetVectorParameterValue` "/Game/SnowSystem/Material/MPC_Capture.MPC_Capture" "CaptureLocation" (`KismetMathLibrary.Conv_VectorToLinearColor` (`self.K2_GetActorLocation`))))

(fn `UserConstructionScript`)